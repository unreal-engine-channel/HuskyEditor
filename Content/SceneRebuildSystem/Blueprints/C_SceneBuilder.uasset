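; C_SceneBuilder is an actor component that rebuilds a saved scene of node pickup items and connecting cables.
; It caches the owner's C_Inventory on BeginPlay, then reads its SavedScene when EventBuildScene fires.
; It spawns items from saved transforms, then cables at the "to" socket's world position, attaching each end to the "from" socket.
; Cable endpoints assume nodes are saved in consecutive pairs, one pair per cable.
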(event `self.ReceiveBeginPlay`
  (set `self.Inventory` (`|GetArrayItem` (`Actor.K2_GetComponentsByClass` (`self.GetOwner`) "/Game/InventorySystem/Components/C_Inventory.C_Inventory_C"))))

(event `EventBuildScene`
  (bind _savedscene (`/Game/InventorySystem/Components/C_Inventory.SavedScene` (`self.Inventory`)))
  ;[0.5 0 0.1865] 初始化不能在EeventBeginPlay中进行
  (set `self.Nodes Transform List` (`/Game/BPLinkSystem/Blueprints/BP_SaveScene.NodesTransformList` _savedscene))
  (set `self.Cables Transform List` (`/Game/BPLinkSystem/Blueprints/BP_SaveScene.CablesTransformList` _savedscene))
  ;[1 0.6336 0] 在场景中生成蓝图节点
  (for _array_element (`self.Nodes Transform List`)
    (bind (_transform _nodeinfo) (break `/Game/BPLinkSystem/Structures/S_SceneBPNodeInfo` _array_element))
    (bind _returnvalue (`|SpawnActorFromClass` "/Game/InventorySystem/Blueprints/BP_PickupItem.BP_PickupItem_C" _transform "Undefined" "OverrideRootScale" null _nodeinfo null))
    (`KismetArrayLibrary.Array_Add` (`self.SpawnPickupItemList`) _returnvalue))
  ;[1 0.6336 0] 在场景中生成Cable
  (for (_array_element_2 _array_index) (`self.Cables Transform List`)
    (bind _returnvalue_2 (* _array_index 2))
    (bind (_frompin _topin) (break `/Game/BPLinkSystem/Structures/S_SceneCableInfo` _array_element_2))
    ;;[0 0.5 0.1586] Cable末端位置
    (bind _returnvalue_3 (`|SpawnActorFromClass` "/Game/BPLinkSystem/Blueprints/BP_Cable.BP_Cable_C" (`KismetMathLibrary.MakeTransform` (`KismetMathLibrary.TransformLocation` (`.Transform_5_9CEA76A948F84EC148CF29BB646707BB` (break `/Game/BPLinkSystem/Structures/S_SceneBPNodeInfo` (`|GetArrayItem` (`self.Nodes Transform List`) (+ _returnvalue_2 1)))) (`.SocketLocation_13_19714364482B841671EF73B009ED6C7D` (break `/Game/BPLinkSystem/Structures/S_SocketInfo` _topin)))) "Undefined" "OverrideRootScale" null false null))
    ;;[0 0.5 0.1586] Cable起始位置
    (`CableComponent.SetAttachEndTo` (`/Game/BPLinkSystem/Blueprints/BP_Cable.Cable` _returnvalue_3) (`|GetArrayItem` (`self.SpawnPickupItemList`) _returnvalue_2) "None" (`.SocketName_16_A37CB3FF4E06A4BD431D499707F2A3F5` (break `/Game/BPLinkSystem/Structures/S_SocketInfo` _frompin)))))