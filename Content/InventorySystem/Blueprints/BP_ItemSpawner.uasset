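; BP_ItemSpawner is an inventory system actor that keeps spawning random pickup items at its own transform.
; A looping one-second timer started on BeginPlay picks a random row from the ItemList data table and passes it as ItemInfo to a new BP_PickupItem.
; Each pickup's static mesh gets a random horizontal velocity scaled by Speed, limited to positive X and Y because the random floats are never negative.
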(event `self.ReceiveBeginPlay`
  (`KismetSystemLibrary.K2_SetTimerDelegate` (delegate `SpawnActor`) 1.0 true))

(event `SpawnActor`
  (bind _returnvalue (`KismetMathLibrary.RandomFloat`))
  (bind _outrownames (`DataTableFunctionLibrary.GetDataTableRowNames` (`self.ItemList`)))
  (bind _returnvalue_2 (`|GetDataTableRow` (`self.ItemList`) (`|GetArrayItem` _outrownames (`KismetMathLibrary.RandomInteger` (`KismetArrayLibrary.Array_Length` _outrownames))))
    (:`then`
      (bind _returnvalue_3 (`|SpawnActorFromClass` "/Game/InventorySystem/Blueprints/BP_PickupItem.BP_PickupItem_C" (`self.GetTransform`) "Undefined" "OverrideRootScale" null _returnvalue_2 null))
      (`PrimitiveComponent.SetPhysicsLinearVelocity` (`/Game/InventorySystem/Blueprints/BP_PickupItem.StaticMesh` _returnvalue_3) (* (`KismetMathLibrary.MakeVector` _returnvalue _returnvalue) (`self.Speed`)) false "None"))))

(fn `UserConstructionScript`)