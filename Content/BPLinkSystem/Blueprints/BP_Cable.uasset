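; BP_Cable is a cable actor that attaches to the player character's right middle-finger socket.
; AttachToPlayer sets the cable component's end to that socket on BP_Character.
; A looping 0.1-second timer started at BeginPlay moves the actor to the socket while HasPlayerPickup is true.
; When the flag is false the timer pauses itself, and its only unpause call sits inside that same callback.
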(event `AttachToPlayer`
  ;[1 0 0.04597] 设置Cable末端指向Player
  (`CableComponent.SetAttachEndTo` (`self.Cable`) (`self.BP_Character`) "None" (`SkinnedMeshComponent.GetSocketBoneName` (`Character.Mesh` (`self.BP_Character`)) "middle_03_rSocket")))

(event `TickAttackToPlayer`
  (bind _attachtimerhandle (`self.AttachTimerHandle`))
  ;[1 0 0.04597] 设置Cable起始端指向Player
  (if (`self.HasPlayerPickup?`)
    (`KismetSystemLibrary.K2_UnPauseTimerHandle` _attachtimerhandle)
    (`self.K2_SetActorLocation` self (`SceneComponent.GetSocketLocation` (`Character.Mesh` (`self.BP_Character`)) "middle_03_rSocket") false false)
    (else
      (`KismetSystemLibrary.K2_PauseTimerHandle` _attachtimerhandle))))

(event `self.ReceiveBeginPlay`
  (bind _asbp_character (cast `/Game/Characters/Blueprints/BP_Character` (`GameplayStatics.GetPlayerCharacter` 0)))
  (set `self.BP_Character` _asbp_character)
  (bind _returnvalue (`KismetSystemLibrary.K2_SetTimerDelegate` (delegate `TickAttackToPlayer`) 0.1 true))
  (set `self.AttachTimerHandle` _returnvalue))

(event `self.ReceiveTick`
  (params (DeltaSeconds :type "Float (single-precision)")))

(fn `UserConstructionScript`)